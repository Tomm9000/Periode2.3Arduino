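; Ghost enemy that roams to random reachable points and reacts to microphone loudness by moving toward the player.
; Louder sound raises walk speed and alters the random offset around the player's location.
; Tick maps player distance to a five-level EMF value for an Arduino over serial, opened on BeginPlay and closed on EndPlay.
; Proximity also drives heartbeat pitch and volume and awards GameMode points.
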(event `self.ReceiveBeginPlay`
  ;[0.0356 0.0356 0.0356] Opens Serial Port
  (bind (_bopened _returnvalue) (`SerialCom.OpenComPortWithFlowControl` (`self.Port`)))
  (if (`SerialCom.IsOpened` _returnvalue)
    (bind _output_get (set `self.MySerialPort` _returnvalue))
    (`SerialCom.Flush` _output_get)
    ;;[0.0356 0.0356 0.0356] Port Has Connected
    (`SerialCom.Println` _returnvalue "WE ARE CONNECTED!!!")
    (`KismetSystemLibrary.PrintString` "PORT IS INITIALIZED!" true true (struct :`R` 0.279227 :`G` 0.745833 :`B` 0.167813 :`A` 1.0) 60.0)
    (else
      ;;[0.0356 0.0356 0.0356 1 16] Error
      (`KismetSystemLibrary.PrintString` "Port is NOT CONNECTED!!!" true true (struct :`R` 1.0 :`A` 1.0) 60.0)))
  ;[0.05098 0.05098 0.05098] Start Loop
  (set `CharacterMovementComponent.MaxWalkSpeed` (* 200.0 (`self.RoamWalkSpeed`)) (`self.CharacterMovement`))
  (`self.Roam` false)
  ;;[0.05098 0.05098 0.05098] Bind Player Event
  (bind _asbp_third_person_character (cast `/Game/ThirdPerson/Blueprints/BP_ThirdPersonCharacter` (`GameplayStatics.GetPlayerCharacter` 0)))
  (add `/Game/ThirdPerson/Blueprints/BP_ThirdPersonCharacter.GameEnd` _asbp_third_person_character (delegate `StopSound`)))

(event `StopSound`
  (`AudioComponent.Stop` (`self.Spotted`))
  (`AudioComponent.Stop` (`self.GhostNoise`))
  (`AudioComponent.Stop` (`self.HeartBeat`)))

(event `Roam`
  (params (FromSound :type Boolean))
  ;[0.05098 0.05098 0.05098] Enemy Moves
  (bind _asbp_third_person_character (cast `/Game/ThirdPerson/Blueprints/BP_ThirdPersonCharacter` (`GameplayStatics.GetPlayerCharacter` 0)))
  (if (`/Game/ThirdPerson/Blueprints/BP_ThirdPersonCharacter.FirstInput` _asbp_third_person_character)
    (if FromSound
      (bind _outvector3 (`self.RandomVector3` (`self.K2_GetActorLocation` _asbp_third_person_character)))
      (`|AIMoveTo` self _outvector3 null
        (:`OnSuccess`
          _))
      (else
        (`|AIMoveTo` self (`NavigationSystemV1.K2_GetRandomReachablePointInRadius` (`self.K2_GetActorLocation`) 2500.0 null null) null
          (:`OnSuccess`
            _))))
    (`KismetSystemLibrary.Delay` 1.0)
    (`self.Roam` false)))

(event `self.ReceiveEndPlay`
  (params (EndPlayReason :type "EEndPlayReason Enum" :default "Destroyed"))
  (bind _myserialport (`self.MySerialPort`))
  ;[0.0382 0.0382 0.0382] Closes Port
  (if (`SerialCom.IsOpened` _myserialport)
    (`SerialCom.Println` _myserialport "THE PROGRAM WAS TERMINATED BY THE USER! ... CLOSSING PORT!")
    (`SerialCom.Close` _myserialport)))

(event `ArduinoRead`
  ;[0.0382 0.0382 0.0382] ArduinoReadPort
  (bind (_bsuccess _returnvalue) (`SerialCom.Readln` (`self.MySerialPort`)))
  (if _bsuccess
    (`KismetSystemLibrary.PrintString` _returnvalue)
    (else
      (`KismetSystemLibrary.PrintString` "AHHHHH")))
  (`KismetSystemLibrary.Delay` 0.1)
  (`self.ArduinoRead`))

(event `self.ReceiveTick`
  (params (DeltaSeconds :type "Float (single-precision)"))
  (bind _sound (`self.Sound`))
  (bind _heartbeat (`self.HeartBeat`))
  (bind _returnvalue (`KismetMathLibrary.Vector_Distance` (`self.K2_GetActorLocation`) (`self.Player`)))
  (bind _returnvalue_2 (- (`self.FallOff`) _returnvalue))
  (bind _returnvalue_3 (and (> _sound 1.0) (or (not (`self.Busy`)) (!= (`self.Player`) (`self.PlayerPref`) :`ErrorTolerance` 10.0))))
  (bind _returnvalue_4 (* DeltaSeconds _returnvalue_2 (`self.PointsMultiplier`)))
  (bind _returnvalue_5 (+ (* _returnvalue_4 0.05) 1.0))
  ;[0.05098 0.05098 0.05098] Update
  ;;[0.05098 0.05098 0.05098] Point System
  (bind _emf (`self.Lights` _returnvalue))
  (if (not (== (`self.EMFPref`) (`self.EMF`)))
    (`SerialCom.WriteInt` (`self.MySerialPort`) _emf))
  (bind _asbp_third_person_game_mode (cast `/Game/ThirdPerson/Blueprints/BP_ThirdPersonGameMode` (`GameplayStatics.GetGameMode`)))
  (`AudioComponent.SetPitchMultiplier` _heartbeat _returnvalue_5)
  (`AudioComponent.SetVolumeMultiplier` _heartbeat _returnvalue_5)
  (if (> _returnvalue_2 0.0)
    (`/Game/ThirdPerson/Blueprints/BP_ThirdPersonGameMode.AddPoints` _asbp_third_person_game_mode _returnvalue_4))
  (set `self.PlayerPref` (`self.Player`))
  (set `self.EMFPref` (`self.EMF`))
  ;;[0.05098 0.05098 0.05098] Reset
  (if _returnvalue_3
    (set `CharacterMovementComponent.MaxWalkSpeed` (* (`self.RoamWalkSpeed`) _sound 200.0) (`self.CharacterMovement`))
    (`self.Roam` _returnvalue_3)))

(event `self.AudioCapture.OnAudioEnvelopeValue`
  (params (EnvelopeValue :type "Float (single-precision)"))
  ;[0.0382 0.0382 0.0382] MicInput
  (set `self.Sound` (* (`self.SoundMult`) EnvelopeValue)))

(fn `AddRand`
  (params (Vector1 :type "Float (double-precision)"))
  (returns (Rand1 :type "Float (double-precision)"))
  (bind _returnvalue (- 10.0 (`self.Sound`)))
  (return (+ Vector1 (`KismetMathLibrary.RandomFloatInRange` _returnvalue (* _returnvalue -1.0)))))

(fn `Lights`
  (params (distance :type "Float (double-precision)"))
  (returns (EMF :type Integer))
  (if (> distance 1200.0)
    (set `self.EMF` 1)
    (elif (> distance 900.0)
      (set `self.EMF` 2)
      (elif (> distance 600.0)
        (set `self.EMF` 3)
        (elif (> distance 300.0)
          (set `self.EMF` 4)
          (else
            (set `self.EMF` 5))))))
  (return (`self.EMF`)))

(fn `RandomVector3`
  (params (Vector3 :type "Vector Structure"))
  (returns (OutVector3 :type "Vector Structure"))
  (bind (_x _y _z) (`KismetMathLibrary.BreakVector3f` Vector3))
  (bind _rand1 (`self.AddRand` _x))
  (bind _rand1_2 (`self.AddRand` _y))
  (return (`KismetMathLibrary.MakeVector` _rand1 _rand1_2 _z)))

(fn `UserConstructionScript`)